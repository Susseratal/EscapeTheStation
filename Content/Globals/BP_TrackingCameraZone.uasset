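; BP_TrackingCameraZone is a trigger zone that switches the player's view to its SelfCamera when BP_Player enters its box.
; Box overlap events store the player reference and set an in-zone flag, and entry sets the view target.
; While the flag is set, Tick moves the camera to the player's Y position, keeping its own X and Z.
; Leaving the box stops tracking but does not change the view target back.
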(event OnComponentBeginOverlap(Box)
  (params (OverlappedComponent :type Primitive%20Component%20Object%20Reference) (OtherActor :type Actor%20Object%20Reference) (OtherComp :type Primitive%20Component%20Object%20Reference) (OtherBodyIndex :type Integer) (bFromSweep :type Boolean) (SweepResult :type Hit%20Result%20Structure%20%28by%20ref%29))
  (bind _asbp_player (Utilities|Casting|CastToBP_Player OtherActor))
  (Game|Player|SetViewTargetwithBlend (Game|GetPlayerController 0) (Variables|Default|GetSelfCamera) 0.0 "VTBlend_Linear" 0.0 false)
  (Variables|Default|SetplayerRef _asbp_player)
  (Variables|Default|SetplayerInZone true))

(event OnComponentEndOverlap(Box)
  (params (OverlappedComponent :type Primitive%20Component%20Object%20Reference) (OtherActor :type Actor%20Object%20Reference) (OtherComp :type Primitive%20Component%20Object%20Reference) (OtherBodyIndex :type Integer))
  (Utilities|Casting|CastToBP_Player OtherActor)
  (Variables|Default|SetplayerInZone false))

(event EventBeginPlay
  (|CallParentFunction) ; This node is disabled and will not be called.\nDrag off pins to build functionality.
)

(event Collision|EventActorBeginOverlap
  (params (OtherActor :type Actor%20Object%20Reference))
  (|CallParentFunction OtherActor) ; This node is disabled and will not be called.\nDrag off pins to build functionality.
)

(event EventTick
  (params (DeltaSeconds :type Float%20%28single-precision%29))
  (bind _selfcamera (Variables|Default|GetSelfCamera))
  (bind _returnvalue (Transformation|GetActorLocation _selfcamera))
  (|CallParentFunction DeltaSeconds)
  (if (Variables|Default|GetplayerInZone)
    (Transformation|SetActorLocation _selfcamera (Math|Vector|MakeVector (.x _returnvalue) (.y (Transformation|GetActorLocation (Variables|Default|GetplayerRef))) (.z _returnvalue)) false false)))

(fn ConstructionScript
  (|CallParentFunction))