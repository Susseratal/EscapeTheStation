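; BP_Door is an interactable sliding door prop that can be locked behind a keycard.
; Interacting while locked opens the player's inventory to request the keycard; using it unlocks the door, refreshes the HUD prompt and toggles the inventory.
; When unlocked, interaction plays the OpenClose timeline from the start to slide the mesh along local X, ignoring input until it finishes.
; EvaluateVerb sets the prompt verb from the lock state, exposed through GetInfo.
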(event EventBeginPlay
  (CallFunction|EvaluateVerb))

(event Collision|EventActorBeginOverlap
  (params (OtherActor :type Actor%20Object%20Reference)))

(event EventTick
  (params (DeltaSeconds :type Float%20%28single-precision%29)))

(event EventInteract
  (params (playerRef :type BP%20Player%20Object%20Reference))
  (if (Variables|Default|Getb_locked)
    (Default|ToggleInventory playerRef true self "/Game/Globals/CollectibleItemData/DBP_Keycard.DBP_Keycard_C" (Variables|Default|Getuid))
    (elif (not (Variables|Default|Getmoving))
      (Variables|Default|Setmoving true)
      (bind _interp (Timeline|Open/Close PlayFromStart)
        (:Update
          (Transformation|SetRelativeLocation (Variables|Default|GetSM_Door) (Math|Vector|Lerp(Vector) "0, 0, 0" "120.000000,0.000000,0.000000" _interp) false false))
        (:Finished
          (Variables|Default|Setmoving false))))))

(event EventPropUsed
  (params (PlayerRef :type BP%20Player%20Object%20Reference))
  (Variables|Default|Setb_locked false)
  (CallFunction|EvaluateVerb)
  (Default|SetPromptData (Variables|/Game/ThirdPerson/Blueprints/BP_Player.BP_Player_C|GetW_Hud PlayerRef) (Variables|Default|GetSelfInfo))
  (Default|ToggleInventory PlayerRef false))

(fn ConstructionScript)

(fn EvaluateVerb
  (if (Variables|Default|Getb_locked)
    (LocalVariables|SetOutVerb "NewEnumerator5")
    (else
      (LocalVariables|SetOutVerb "NewEnumerator6")))
  (Utilities|Struct|SetmembersinDS_InteractionData (Variables|Default|GetSelfInfo) (Utilities|Array|MakeArray (LocalVariables|GetOutVerb))))

(fn GetInfo
  (return (Variables|Default|GetSelfInfo)))