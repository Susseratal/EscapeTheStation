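; BP_Key is a keycard prop that the player can interact with to pick up into their inventory.
; GetInfo supplies interaction data with the Keycard name and a single verb.
; Interact checks for a full inventory, calls PickUpItem on the player and destroys the actor on success.
; A full inventory or failed pickup shows a notification on the player's HUD widget instead.
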(event EventBeginPlay
  (|CallParentFunction) ; This node is disabled and will not be called.\nDrag off pins to build functionality.
)

(event Collision|EventActorBeginOverlap
  (params (OtherActor :type Actor%20Object%20Reference))
  (|CallParentFunction OtherActor) ; This node is disabled and will not be called.\nDrag off pins to build functionality.
)

(event EventTick
  (params (DeltaSeconds :type Float%20%28single-precision%29))
  (|CallParentFunction DeltaSeconds) ; This node is disabled and will not be called.\nDrag off pins to build functionality.
)

(event EventInteract
  (params (playerRef :type BP%20Player%20Object%20Reference))
  (bind _w_hud (Variables|/Game/ThirdPerson/Blueprints/BP_Player.BP_Player_C|GetW_Hud playerRef))
  (if (Default|IsInventoryFull playerRef)
    (Default|AddNotification _w_hud "You have no space")
    (else
      (bind _pickedup (Default|PickUpItem playerRef self))
      (if _pickedup
        (Actor|DestroyActor)
        (else
          (Default|AddNotification _w_hud "Error picking up object"))))))

(fn ConstructionScript
  (|CallParentFunction))

(fn GetInfo
  (return (Utilities|Struct|MakeDS_InteractionData "Keycard" (Utilities|Array|MakeArray "NewEnumerator0"))))